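; BP_Projectile is a homing projectile that chases EnemyToAttack and damages it on arrival.
; Each Tick it moves toward the target at Speed without sweeping, using a distance tolerance instead of collision to detect the hit.
; On impact it spawns an effect, sends Damage through an interface message and destroys itself.
; If the target becomes invalid, it flies to the cached LastLocation and bursts there without dealing damage.
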(event `self.ReceiveBeginPlay`)

(event `self.ReceiveTick`
  (params (DeltaSeconds :type "Float (single-precision)"))
  (bind _returnvalue (`self.K2_GetActorLocation`))
  (bind _returnvalue_2 (`self.K2_GetActorLocation`))
  (bind _enemytoattack (`self.EnemyToAttack`))
  (bind _lastlocation (`self.LastLocation`))
  (bind _enemytoattack_2 (`self.EnemyToAttack`))
  (bind _returnvalue_3 (`self.K2_GetActorLocation` _enemytoattack))
  (`/Engine/EditorBlueprintResources/StandardMacros.IsValid` _enemytoattack
    (:`Is Valid`
      (if (== _returnvalue_3 _returnvalue_2 :`ErrorTolerance` 20.0)
        (`GameplayStatics.SpawnEmitterAtLocation` (`self.Impact_SFX`) _returnvalue_2)
        (`/Engine/EditorBlueprintResources/StandardMacros.IsValid` _enemytoattack_2
          (:`Is Valid`
            (message `/Game/Blueprints/Units/AI/DamageInterface.TakeDamageInterface` _enemytoattack_2 (`self.Damage`))
            (`self.K2_DestroyActor`)))
        (else
          (`self.K2_AddActorWorldOffset` (* (`KismetMathLibrary.Normal` (- _returnvalue_3 _returnvalue_2)) (* DeltaSeconds (`self.Speed`))))
          (`/Engine/EditorBlueprintResources/StandardMacros.IsValid` _enemytoattack
            (:`Is Valid`
              (set `self.LastLocation` _returnvalue_3))))))
    (:`Is Not Valid`
      (if (== _lastlocation _returnvalue :`ErrorTolerance` 1.0)
        (`GameplayStatics.SpawnEmitterAtLocation` (`self.Impact_SFX`) _returnvalue)
        (`self.K2_DestroyActor`)
        (else
          (`self.K2_AddActorWorldOffset` (* (`KismetMathLibrary.Normal` (- _lastlocation _returnvalue)) (* DeltaSeconds (`self.Speed`)))))))))

(fn `UserConstructionScript`)