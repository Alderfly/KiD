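; Defensive tower building that automatically shoots projectiles at characters of other teams within its attack radius.
; Construction reads the Tower data table row for health, armor, fire rate and radius, then sizes the range ring and detection sphere.
; Sphere overlaps maintain an enemy list; a DoOnce-gated looping timer spawns BP_Projectile targeting the first entry and stops when the list empties.
; BeginPlay also sets the tower's widget icon.
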(event `self.ReceiveBeginPlay`
  (`parent.ReceiveBeginPlay`)
  (`KismetArrayLibrary.Array_Clear` (`self.ListOfEnemies`))
  (bind _asw_entity_icon (cast `/Game/Blueprints/UI/W_EntityIcon` (`WidgetComponent.GetUserWidgetObject` (`self.WidgetIcon`))))
  (`Image.SetBrushFromTexture` (`/Game/Blueprints/UI/W_EntityIcon.Image_0` _asw_entity_icon) "/Game/Blueprints/UI/Assets/Buttons/Tower_Btn.Tower_Btn" false))

(event `self.SphereDetectionRadius.OnComponentBeginOverlap`
  (params (OverlappedComponent :type "PrimitiveComponent Object Reference") (OtherActor :type "Actor Object Reference") (OtherComp :type "PrimitiveComponent Object Reference") (OtherBodyIndex :type Integer) (bFromSweep :type Boolean) (SweepResult :type "HitResult Structure (by ref)"))
  (bind _asbp_base_character (cast `/Game/Blueprints/Units/BP_BaseCharacter` OtherActor))
  (`/Engine/EditorBlueprintResources/StandardMacros.IsValid` _asbp_base_character
    (:`Is Valid`
      (if (`|EnumInequality` (`KID_Character.Team` _asbp_base_character) (`self.Team`))
        (`KismetArrayLibrary.Array_Add` (`self.ListOfEnemies`) _asbp_base_character)
        (`/Engine/EditorBlueprintResources/StandardMacros.DoOnce` false :!label _label
          (:`Completed`
            (`KismetSystemLibrary.K2_SetTimer` null "AttackEnemy" (`self.FireRate`) true)))))))

(event `self.SphereDetectionRadius.OnComponentEndOverlap`
  (params (OverlappedComponent :type "PrimitiveComponent Object Reference") (OtherActor :type "Actor Object Reference") (OtherComp :type "PrimitiveComponent Object Reference") (OtherBodyIndex :type Integer))
  (bind _listofenemies (`self.ListOfEnemies`))
  (bind _asbp_base_character (cast `/Game/Blueprints/Units/BP_BaseCharacter` OtherActor))
  (`KismetArrayLibrary.Array_RemoveItem` _listofenemies _asbp_base_character)
  (if (== (`KismetArrayLibrary.Array_Length` _listofenemies) 0)
    (`KismetSystemLibrary.K2_ClearTimer` null "AttackEnemy")
    (goto _label :!via `Reset`)))

(fn `AttackEnemy`
  (bind _listofenemies (`self.ListOfEnemies`))
  (if (!= (`KismetArrayLibrary.Array_Length` _listofenemies) 0)
    (bind _returnvalue (`|SpawnActorFromClass` "/Game/Blueprints/Projectiles/BP_Projectile.BP_Projectile_C" (`SceneComponent.K2_GetComponentToWorld` (`self.Shooting point`)) "Undefined" "OverrideRootScale" null null))
    (set `/Game/Blueprints/Projectiles/BP_Projectile.EnemyToAttack` (`|GetArrayItem` _listofenemies) _returnvalue)
    (`KismetSystemLibrary.PrintString` "spawned")))

(fn `UserConstructionScript`
  (`parent.UserConstructionScript`)
  (bind _returnvalue (`|GetDataTableRow` "/Game/Blueprints/Miscellaneous/CostsDataTable.CostsDataTable" "Tower")
    (:`then`
      (bind (_name _cost _health _armor _attack _reloadtime _attackradius) (break `/Game/Blueprints/Miscellaneous/ESGameData` _returnvalue))
      (set `self.StartingHealth` _health)
      (set `self.Armor` _armor)
      (set `self.FireRate` _reloadtime)
      (bind _output_get (set `self.AttackRadius` _attackradius))
      (bind _returnvalue_2 (`KismetMathLibrary.Conv_IntToDouble` _output_get))
      (`SceneComponent.SetWorldScale3D` (`self.Ring`) (`KismetMathLibrary.MakeVector` 1.0 _returnvalue_2 _returnvalue_2))
      (`SphereComponent.SetSphereRadius` (`self.SphereDetectionRadius`) (`KismetMathLibrary.Conv_IntToDouble` _attackradius) true))))