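; Base building actor with a team-colored mesh, an overhead health bar widget and an interface entry point for damage.
; The construction script creates a dynamic M_TeamBuilding material and sets TeamColor from the Team value.
; After a short delay at BeginPlay, it registers itself as the W_HealthBar owner and flags it as a building.
; TakeDamageInterface forwards the amount to ApplyDamage on itself, with no health handling in these graphs.
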(event `self.ReceiveBeginPlay`
  (`KismetSystemLibrary.Delay` 0.2)
  (bind _asw_health_bar (cast `/Game/Blueprints/UI/W_HealthBar` (`WidgetComponent.GetUserWidgetObject` (`self.Widget`))))
  (set `/Game/Blueprints/UI/W_HealthBar.Owner` self _asw_health_bar)
  (set `/Game/Blueprints/UI/W_HealthBar.isBuilding` true _asw_health_bar))

(event `/Game/Blueprints/Units/AI/DamageInterface.TakeDamageInterface`
  (params (Amount :type "Float (single-precision)"))
  (`GameplayStatics.ApplyDamage` self Amount))

(fn `UserConstructionScript`
  (bind _buildingmesh (`self.BuildingMesh`))
  (switch `ETeam` (`self.Team`)
    (:`None`
      (bind _returnvalue (`PrimitiveComponent.CreateDynamicMaterialInstance` _buildingmesh 0 "/Game/Environment/Materials/M_TeamBuilding.M_TeamBuilding"))
      (`MaterialInstanceDynamic.SetVectorParameterValue` _returnvalue "TeamColor" (struct :`R` 1.0 :`G` 1.0 :`B` 1.0 :`A` 1.0)))
    (:`Player`
      (bind _returnvalue_2 (`PrimitiveComponent.CreateDynamicMaterialInstance` _buildingmesh 0 "/Game/Environment/Materials/M_TeamBuilding.M_TeamBuilding"))
      (`MaterialInstanceDynamic.SetVectorParameterValue` _returnvalue_2 "TeamColor" (struct :`B` 1.0 :`A` 1.0)))
    (:`Team1`
      (bind _returnvalue_3 (`PrimitiveComponent.CreateDynamicMaterialInstance` _buildingmesh 0 "/Game/Environment/Materials/M_TeamBuilding.M_TeamBuilding"))
      (`MaterialInstanceDynamic.SetVectorParameterValue` _returnvalue_3 "TeamColor" (struct :`R` 1.0 :`A` 1.0)))))