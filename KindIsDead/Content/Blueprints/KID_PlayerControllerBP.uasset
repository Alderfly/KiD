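; Player controller that shows the mouse cursor and moves the controlled pawn as a camera, by edge scrolling or drag panning.
; Each Tick, UpdateCamera switches on an input state of None, Hold or Scroll.
; A cursor in the outer 10% of the viewport adds movement input along its direction from screen centre.
; Holding PanCamera offsets the pawn in XY by the delta between cursor traces, keeping the grabbed point under the cursor.
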(event `self.ReceiveBeginPlay`
  (set `self.bShowMouseCursor` true)
  (`WidgetBlueprintLibrary.SetInputMode_GameAndUIEx` self null "DoNotLock" false))

(event `self.ReceiveTick`
  (params (DeltaSeconds :type "Float (single-precision)"))
  (set `self.DeltaTime` DeltaSeconds)
  (`self.UpdateCamera`))

(event `UpdateCamera`
  (bind _returnvalue (`self.K2_GetPawn`))
  ;[1 1 1] Update Camera Position
  (switch `/Game/Blueprints/Miscellaneous/EInputType` (`self.ECurrentInputState`)
    (:`NewEnumerator0`
      (bind _drag (`self.IsScrolling` :!label _label))
      (if (`|EnumInequality` _drag "NewEnumerator0")
        (bind _direction (`self.GetScrollDirection`))
        (`Pawn.AddMovementInput` (`self.K2_GetPawn`) _direction 1.0 false)
        (set `self.ECurrentInputState` "NewEnumerator3")))
    (:`NewEnumerator2`
      (if (`self.isScrollingCamera`)
        (bind _delta (`self.OnSwipeUpdate`))
        (`self.K2_SetActorLocation` _returnvalue (+ _delta (`self.K2_GetActorLocation` _returnvalue)) false false)))
    (:`NewEnumerator3`
      (goto _label))))

(event `InputAction|PanCamera`
  (params (Key :type "Key Structure"))
  (:`Pressed`
    (`self.OnSwipeStarted`)
    (set `self.ECurrentInputState` "NewEnumerator2")
    (set `self.isScrollingCamera` true))
  (:`Released`
    (`self.OnSwipeEnded`)
    (set `self.ECurrentInputState` "NewEnumerator0")))

(fn `GetScrollDirection`
  (returns (Direction :type "Vector Structure"))
  (bind (_locationx _locationy) (`self.GetMousePosition`))
  (return (`KismetMathLibrary.MakeVector` (* -1 (.y (`KismetMathLibrary.ClampVectorSize` (* (`KismetMathLibrary.Conv_Vector2DToVector` (- (`KismetMathLibrary.MakeVector2D` _locationx _locationy) (/ (`WidgetLayoutLibrary.GetViewportSize`) 2.0))) 1) 0.2 1.0))) (* 1 (.x (`KismetMathLibrary.ClampVectorSize` (* (`KismetMathLibrary.Conv_Vector2DToVector` (- (`KismetMathLibrary.MakeVector2D` _locationx _locationy) (/ (`WidgetLayoutLibrary.GetViewportSize`) 2.0))) 1) 0.2 1.0))))))

(fn `IsScrolling`
  (returns (Drag :type "/Game/Blueprints/Miscellaneous/ECameraScroll Enum"))
  (locals (LocalDrag :type "/Game/Blueprints/Miscellaneous/ECameraScroll Enum"))
  (bind (_locationx _locationy) (`self.GetMousePosition`))
  (bind (_locationx_2 _locationy_2) (`self.GetMousePosition`))
  (bind (_locationx_3 _locationy_3) (`self.GetMousePosition`))
  (bind (_x _y) (`KismetMathLibrary.BreakVector2D` (`WidgetLayoutLibrary.GetViewportSize`)))
  (bind (_x_2 _y_2) (`KismetMathLibrary.BreakVector2D` (`WidgetLayoutLibrary.GetViewportSize`)))
  (bind _returnvalue (< _locationx (* _x 0.1)))
  (bind _returnvalue_2 (< _locationy (* _y 0.1)))
  (`|ExecutionSequence`
    (:`then_0`
      (if _returnvalue
        (set `local.LocalDrag` "NewEnumerator1")))
    (:`then_1`
      (if (and (not _returnvalue) (> _locationx_2 (* _x_2 0.9)))
        (set `local.LocalDrag` "NewEnumerator2")))
    (:`then_2`
      (if _returnvalue_2
        (set `local.LocalDrag` "NewEnumerator4")))
    (:`then_3`
      (if (and (not _returnvalue_2) (> _locationy_2 (* _y_2 0.9)))
        (set `local.LocalDrag` "NewEnumerator3")))
    (:`then_4`
      (if (and (== _locationx_3 0.0) (== _locationy_3 0.0))
        (set `local.LocalDrag` "NewEnumerator0")))
    (:`then_5`
      (return (`local.LocalDrag`)))))

(fn `OnSwipeEnded`
  (set `self.EndSwipeCoordinates` (`.Location` (`GameplayStatics.BreakHitResult` (`self.GetHitResultUnderCursorByChannel` "TraceTypeQuery3"))))
  (set `self.StartSwipeCoordinates` (0.0 0.0 0.0)))

(fn `OnSwipeStarted`
  (set `self.StartSwipeCoordinates` (`.Location` (`GameplayStatics.BreakHitResult` (`self.GetHitResultUnderCursorByChannel` "TraceTypeQuery3")))))

(fn `OnSwipeUpdate`
  (returns (Delta :type "Vector Structure"))
  (locals (LocalNewSwipeCoordinates :type "Vector Structure") (LocalDelta :type "Vector Structure"))
  (set `local.LocalNewSwipeCoordinates` (`.Location` (`GameplayStatics.BreakHitResult` (`self.GetHitResultUnderCursorByChannel` "TraceTypeQuery3"))))
  (bind _output_get (set `local.LocalDelta` (`KismetMathLibrary.MakeVector` (.x (- (`self.StartSwipeCoordinates`) (`local.LocalNewSwipeCoordinates`))) (.y (- (`self.StartSwipeCoordinates`) (`local.LocalNewSwipeCoordinates`))))))
  (return _output_get))

(fn `UserConstructionScript`)