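; BP_Archer is a ranged unit that attacks enemies by shooting projectiles.
; On BeginPlay it runs the BT_Archer behavior tree through its BP_CharacterAIController and sets its W_EntityIcon widget image to the archer button texture.
; AttackEnemy spawns a scaled-down BP_Projectile at the ShootingPoint component and passes it the enemy to attack.
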(event `self.ReceiveBeginPlay`
  (`parent.ReceiveBeginPlay`)
  (bind _asbp_character_aicontroller (cast `/Game/Blueprints/BP_CharacterAIController` (`self.GetController`)))
  (`AIController.RunBehaviorTree` _asbp_character_aicontroller "/Game/Blueprints/Units/AI/BT_Archer.BT_Archer")
  (bind _asw_entity_icon (cast `/Game/Blueprints/UI/W_EntityIcon` (`WidgetComponent.GetUserWidgetObject` (`self.Widget`))))
  (`Image.SetBrushFromTexture` (`/Game/Blueprints/UI/W_EntityIcon.Image_0` _asw_entity_icon) "/Game/Blueprints/UI/Assets/Buttons/Archer_Btn.Archer_Btn" false))

(fn `AttackEnemy`
  (params (Enemy :type "Actor Object Reference"))
  (bind _returnvalue (`|SpawnActorFromClass` "/Game/Blueprints/BP_Projectile.BP_Projectile_C" (`KismetMathLibrary.MakeTransform` (`SceneComponent.K2_GetComponentLocation` (`self.Shooting point`)) (struct) (0.2 0.2 0.2)) "Undefined" "OverrideRootScale" null null))
  (set `/Game/Blueprints/BP_Projectile.EnemyToAttack` Enemy _returnvalue))

(fn `UserConstructionScript`
  (`parent.UserConstructionScript`))