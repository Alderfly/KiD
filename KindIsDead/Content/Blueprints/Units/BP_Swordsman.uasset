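; Swordsman unit, a child Blueprint that configures its combat stats, AI and icon on top of its parent's logic.
; The construction script reads the Swordsman row from CostsDataTable for health, armor, attack, reload, speed and attack radius, which also sizes the Ring and Sphere components.
; After a short delay on BeginPlay, it starts BT_Swordsman on its BP_CharacterAIController, then sets the Swordsman image on its W_EntityIcon widget.
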(event `self.ReceiveBeginPlay`
  (`parent.ReceiveBeginPlay`)
  (`KismetSystemLibrary.Delay` 0.2)
  (bind _asbp_character_aicontroller (cast `/Game/Blueprints/BP_CharacterAIController` (`self.GetController`)))
  (`AIController.RunBehaviorTree` _asbp_character_aicontroller "/Game/Blueprints/Units/AI/BT_Swordsman.BT_Swordsman")
  (bind _asw_entity_icon (cast `/Game/Blueprints/UI/W_EntityIcon` (`WidgetComponent.GetUserWidgetObject` (`self.Widget`))))
  (`Image.SetBrushFromTexture` (`/Game/Blueprints/UI/W_EntityIcon.Image_0` _asw_entity_icon) "/Game/Blueprints/UI/Assets/Buttons/Swordsman_Btn.Swordsman_Btn" false))

(fn `UserConstructionScript`
  (`parent.UserConstructionScript`)
  (bind _returnvalue (`|GetDataTableRow` "/Game/Blueprints/Miscellaneous/CostsDataTable.CostsDataTable" "Swordsman")
    (:`then`
      (bind (_name _cost _health _armor _attack _reloadtime _attackradius _projectilespeed _speed) (break `/Game/Blueprints/Miscellaneous/ESGameData` _returnvalue))
      (set `self.StartingHealth` _health)
      (set `self.Armor` _armor)
      (set `self.Attack` _attack)
      (set `self.ReloadTime` _reloadtime)
      (bind _output_get (set `self.AttackRadius` _attackradius))
      (bind _returnvalue_2 (`KismetMathLibrary.Conv_IntToDouble` _output_get))
      (`SceneComponent.SetWorldScale3D` (`self.Ring`) (`KismetMathLibrary.MakeVector` 1.0 _returnvalue_2 _returnvalue_2))
      (set `self.Speed` _speed)
      (`SphereComponent.SetSphereRadius` (`self.Sphere`) (`KismetMathLibrary.Conv_IntToDouble` _attackradius) true))))