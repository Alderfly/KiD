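; BP_BaseCharacter is a team-based unit with a health bar widget and a list of enemy units in range to attack.
; After a short delay on BeginPlay it links the W_HealthBar to itself and, if already Placed, calls Initialize, which enables collision and colors the bar by team.
; Sphere overlaps add opposing-team characters to UnitsToAttack and remove them on exit, while TakeDamageInterface forwards damage through ApplyDamage.
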(event `self.ReceiveBeginPlay`
  (`KismetSystemLibrary.Delay` 0.2)
  (bind _asw_health_bar (cast `/Game/Blueprints/UI/W_HealthBar` (`WidgetComponent.GetUserWidgetObject` (`self.Health_Widget`))))
  (set `/Game/Blueprints/UI/W_HealthBar.Owner` self _asw_health_bar)
  (set `/Game/Blueprints/UI/W_HealthBar.isBuilding` false _asw_health_bar)
  (`KismetArrayLibrary.Array_Clear` (`self.UnitsToAttack`))
  (if (`self.bPlaced`)
    (`self.Initialize` (`self.Team`))))

(event `/Game/Blueprints/Units/AI/DamageInterface.TakeDamageInterface`
  (params (Amount :type "Float (single-precision)"))
  (`GameplayStatics.ApplyDamage` self Amount))

(event `self.Sphere.OnComponentBeginOverlap`
  (params (OverlappedComponent :type "PrimitiveComponent Object Reference") (OtherActor :type "Actor Object Reference") (OtherComp :type "PrimitiveComponent Object Reference") (OtherBodyIndex :type Integer) (bFromSweep :type Boolean) (SweepResult :type "HitResult Structure (by ref)"))
  (bind _asbp_base_character (cast `/Game/Blueprints/Units/BP_BaseCharacter` OtherActor))
  (if (`|EnumInequality` (`KID_Character.Team` _asbp_base_character) (`self.Team`))
    (`KismetArrayLibrary.Array_Add` (`self.UnitsToAttack`) _asbp_base_character)))

(event `self.Sphere.OnComponentEndOverlap`
  (params (OverlappedComponent :type "PrimitiveComponent Object Reference") (OtherActor :type "Actor Object Reference") (OtherComp :type "PrimitiveComponent Object Reference") (OtherBodyIndex :type Integer))
  (bind _asbp_base_character (cast `/Game/Blueprints/Units/BP_BaseCharacter` OtherActor))
  (`KismetArrayLibrary.Array_RemoveItem` (`self.UnitsToAttack`) _asbp_base_character))

(fn `Initialize`
  (params (Team :type "ETeam Enum" :default "None"))
  (bind _returnvalue (`WidgetComponent.GetUserWidgetObject` (`self.Health_Widget`)))
  (bind _output_get (set `self.Team` Team))
  (`PrimitiveComponent.SetCollisionEnabled` (`self.Sphere`) "QueryOnly")
  (`PrimitiveComponent.SetCollisionEnabled` (`self.CapsuleComponent`) "QueryAndPhysics")
  (switch `ETeam` _output_get
    (:`Player`
      (bind _asw_health_bar (cast `/Game/Blueprints/UI/W_HealthBar` _returnvalue))
      (`ProgressBar.SetFillColorAndOpacity` (`/Game/Blueprints/UI/W_HealthBar.ProgressBar_0` _asw_health_bar) (struct :`R` 0.199474 :`G` 0.229393 :`B` 1.0 :`A` 1.0)))
    (:`Team1`
      (bind _asw_health_bar_2 (cast `/Game/Blueprints/UI/W_HealthBar` _returnvalue))
      (`ProgressBar.SetFillColorAndOpacity` (`/Game/Blueprints/UI/W_HealthBar.ProgressBar_0` _asw_health_bar_2) (struct :`R` 1.0 :`A` 1.0)))))

(fn `UserConstructionScript`)