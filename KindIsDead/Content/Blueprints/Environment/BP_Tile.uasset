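; BP_Tile is an environment tile actor whose TileType sets it up as either empty or ground.
; The construction script switches on that type to set the tile mesh's material and in-game visibility and the plane collision's responses.
; Empty tiles are hidden in game and block only one custom trace channel, while ground tiles are visible and block all channels.
; The event graph holds no logic.
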(fn `UserConstructionScript`
  (bind _tilemesh (`self.TileMesh`))
  (bind _tilemesh_2 (`self.TileMesh`))
  (bind _planecollision (`self.PlaneCollision`))
  (switch `ETileType` (`self.TileType`)
    (:`Empty`
      (`PrimitiveComponent.SetMaterial` _tilemesh 0 (`self.EmtyMaterial`))
      (`SceneComponent.SetHiddenInGame` _tilemesh_2 true false)
      (`PrimitiveComponent.SetCollisionResponseToAllChannels` _planecollision "ECR_Ignore")
      (`PrimitiveComponent.SetCollisionResponseToChannel` (`self.PlaneCollision`) "ECC_GameTraceChannel1" "ECR_Block"))
    (:`Ground`
      (`PrimitiveComponent.SetMaterial` _tilemesh 0 (`self.GroundMaterial`))
      (`SceneComponent.SetHiddenInGame` _tilemesh_2 false false)
      (`PrimitiveComponent.SetCollisionResponseToAllChannels` _planecollision "ECR_Block"))))