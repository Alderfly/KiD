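; KID_SpectatorPawn is a spectator pawn with a spring arm camera that the player can zoom in and out.
; Zoom inputs step a desired zoom distance up or down within min and max limits.
; Each tick interpolates the current zoom toward that target with FInterpTo and applies it as the spring arm length, starting at the desired value on BeginPlay.
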(event `SetDefaultCameraSettings`
  (bind _output_get (set `self.CurrentCameraZoom` (`self.DesiredCameraZoom`)))
  (set `SpringArmComponent.TargetArmLength` _output_get (`self.SpringArm`)))

(event `self.ReceiveBeginPlay`
  (`self.SetDefaultCameraSettings`))

(event `self.ReceiveTick`
  (params (DeltaSeconds :type "Float (single-precision)"))
  (set `self.DeltaTime` DeltaSeconds)
  (`self.UpdateCameraZoom`))

(event `InputAction|ZoomIn`
  (params (Key :type "Key Structure"))
  ;[1 1 1] Zoom inputs
  (:`Pressed`
    (set `self.DesiredCameraZoom` (`KismetMathLibrary.FClamp` (+ (`self.DesiredCameraZoom`) 50.0) (`self.MinCameraZoom`) (`self.MaxCameraZoom`)))))

(event `InputAction|ZoomOut`
  (params (Key :type "Key Structure"))
  ;[1 1 1] Zoom inputs
  (:`Pressed`
    (set `self.DesiredCameraZoom` (`KismetMathLibrary.FClamp` (+ (`self.DesiredCameraZoom`) -50.0) (`self.MinCameraZoom`) (`self.MaxCameraZoom`)))))

(event `UpdateCameraZoom`
  ;[1 1 1] Update Camera Zoom
  (if (not (== (`self.CurrentCameraZoom`) (`self.DesiredCameraZoom`)))
    (bind _output_get (set `self.CurrentCameraZoom` (`KismetMathLibrary.FInterpTo` (`self.CurrentCameraZoom`) (`self.DesiredCameraZoom`) (`self.DeltaTime`) (`self.CameraZoomSpeed`))))
    (set `SpringArmComponent.TargetArmLength` _output_get (`self.SpringArm`))))

(fn `UserConstructionScript`)