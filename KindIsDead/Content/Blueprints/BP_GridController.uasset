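; BP_GridController is the Team1 AI commander that spawns units, roads and towers.
; A looping timer compares Player and Team1 character counts to shift ThreatLevel and order weights, then prunes and prioritizes the order pool by threat.
; An empty pool gets a weighted-random order; otherwise the top order spawns if energy covers its DataTable cost.
; Pikeman and Cavalry reuse Swordsman and Archer, and Mine rolls produce Tower orders.
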(event `UPDATE THREAT LEVEL`
  (bind _threatlevel (`self.ThreatLevel`))
  (bind (_ordersweights_archer _ordersweights_swordsman _ordersweights_pikeman _ordersweights_cavalry _ordersweights_road) (break `/Game/Blueprints/Miscellaneous/ESOrderWeight` (`self.OrdersWeights`)))
  (bind (_ordersweights_archer_2 _ordersweights_swordsman_2 _ordersweights_pikeman_2 _ordersweights_cavalry_2 _ordersweights_road_2) (break `/Game/Blueprints/Miscellaneous/ESOrderWeight` (`self.OrdersWeights`)))
  ;[1 1 1] Update Threat Level
  (bind (_playerbs _team1bs _playerchs _team1chs) (`self.GetAllArrays`))
  (`/Engine/EditorBlueprintResources/StandardMacros.CompareInt` (`KismetArrayLibrary.Array_Length` _playerchs) (`KismetArrayLibrary.Array_Length` _team1chs)
    (:`>`
      (bind _result (`/Engine/EditorBlueprintResources/StandardMacros.IncrementInt` _threatlevel)
        (:`  `
          (`|ExecutionSequence`
            (:`then_0`
              (set `self.OrdersWeights` (make `/Game/Blueprints/Miscellaneous/ESOrderWeight` _result _result _result _result 50 _result)))
            (:`then_1`
              (bind _result_2 (`/Engine/EditorBlueprintResources/StandardMacros.DecrementInt` _ordersweights_road_2)
                (:`  `
                  (set `self.OrdersWeights` (make `/Game/Blueprints/Miscellaneous/ESOrderWeight` 50 50 50 50 _result_2 50 _result_2)))))))))
    (:`==`
      (bind _result_3 (`/Engine/EditorBlueprintResources/StandardMacros.DecrementInt` _threatlevel :!label _label)
        (:`  `
          (`|ExecutionSequence`
            (:`then_0`
              (set `self.OrdersWeights` (make `/Game/Blueprints/Miscellaneous/ESOrderWeight` _result_3 _result_3 _result_3 _result_3 50 _result_3)))
            (:`then_1`
              (bind _result_4 (`/Engine/EditorBlueprintResources/StandardMacros.IncrementInt` _ordersweights_road)
                (:`  `
                  (set `self.OrdersWeights` (make `/Game/Blueprints/Miscellaneous/ESOrderWeight` 50 50 50 50 _result_4 50 _result_4)))))))))
    (:`<`
      (goto _label))))

(event `self.ReceiveBeginPlay`
  (bind _askid_game_mode (cast `/Game/Blueprints/KID_GameMode` (`GameplayStatics.GetGameMode`)))
  (set `self.GameMode_Ref` _askid_game_mode)
  (`KismetSystemLibrary.K2_SetTimer` null "Main" (`self.AIGoalsUpdateTime`) true))

(event `self.ReceiveTick`
  (params (DeltaSeconds :type "Float (single-precision)")))

(event `Main`
  (`self.UPDATE THREAT LEVEL`)
  (`self.UpdatePool`)
  (if (== (`KismetArrayLibrary.Array_Length` (`self.SpawnEntitiesPool`)) 0)
    (`self.AddOrder`)
    (else
      (`self.ExecuteOrder`))))

(fn `AddOrder`
  (locals (hasOrder :type Boolean) (L_UnitPosition :type "Vector Structure" :default (0.0 0.0 0.0)))
  (set `local.hasOrder` false)
  (bind _ordernumber (`self.RollOrders`))
  (switch `int` _ordernumber
    (:`0`
      ;[1 1 1] Units Spawn Orders
      (bind _position (`self.GetUnitPositionToSpawn`))
      (`KismetArrayLibrary.Array_Add` (`self.SpawnEntitiesPool`) (make `/Game/Blueprints/Miscellaneous/ESOrder` "NewEnumerator0" _position (`self.ThreatLevel`))))
    (:`1`
      (bind _position_2 (`self.GetUnitPositionToSpawn`))
      (`KismetArrayLibrary.Array_Add` (`self.SpawnEntitiesPool`) (make `/Game/Blueprints/Miscellaneous/ESOrder` "NewEnumerator1" _position_2 (`self.ThreatLevel`))))
    (:`2`
      (bind _position_3 (`self.GetUnitPositionToSpawn`))
      (`KismetArrayLibrary.Array_Add` (`self.SpawnEntitiesPool`) (make `/Game/Blueprints/Miscellaneous/ESOrder` "NewEnumerator3" _position_3 (`self.ThreatLevel`))))
    (:`3`
      (bind _position_4 (`self.GetUnitPositionToSpawn`))
      (`KismetArrayLibrary.Array_Add` (`self.SpawnEntitiesPool`) (make `/Game/Blueprints/Miscellaneous/ESOrder` "NewEnumerator4" _position_4 (`self.ThreatLevel`))))
    (:`4`
      ;[1 1 1] Road To Spawn
      (bind _tile (`self.GetTileToSpawn`))
      (set `self.TileToSpawn` _tile)
      (`KismetArrayLibrary.Array_Add` (`self.SpawnEntitiesPool`) (make `/Game/Blueprints/Miscellaneous/ESOrder` "NewEnumerator2" (0.0 0.0 0.0) (`self.ThreatLevel`))))
    (:`5`
      ;[1 1 1] Tower To Spawn
      (bind _position_5 (`self.GetTowerPositionToSpawn` :!label _label))
      (`KismetArrayLibrary.Array_Add` (`self.SpawnEntitiesPool`) (make `/Game/Blueprints/Miscellaneous/ESOrder` "NewEnumerator5" _position_5 (`self.ThreatLevel`))))
    (:`6`
      (goto _label))))

(fn `ExecuteOrder`
  (locals (L_Position :type "Vector Structure"))
  (bind _tiletospawn (`self.TileToSpawn`))
  (bind (_spawntype _position) (break `/Game/Blueprints/Miscellaneous/ESOrder` (`|GetArrayItem` (`self.SpawnEntitiesPool`))))
  (set `local.L_Position` _position)
  (switch `/Game/Blueprints/Miscellaneous/ESpawnEntities` _spawntype
    (:`NewEnumerator0`
      ;[1 1 1] Spawn Archer
      (bind _returnvalue (`|GetDataTableRow` "/Game/Blueprints/Miscellaneous/CostsDataTable.CostsDataTable" "Archer")
        (:`then`
          (bind _bresult (`/Game/Blueprints/KID_GameMode.RemoveEnergy` (`self.GameMode_Ref`) (`.Cost_5_B90C82224BB4A7B264F7EB84BBB7EBB3` (break `/Game/Blueprints/Miscellaneous/ESGameData` _returnvalue)) "Team1"))
          (if _bresult
            (bind _returnvalue_2 (`|SpawnActorFromClass` "/Game/Blueprints/Units/BP_Archer.BP_Archer_C" (`KismetMathLibrary.Conv_VectorToTransform` (`local.L_Position`)) "Undefined" "OverrideRootScale" null null))
            (`/Game/Blueprints/Units/BP_BaseCharacter.Initialize` _returnvalue_2 "Team1")
            (`KismetArrayLibrary.Array_Remove` (`self.SpawnEntitiesPool`))
            (else
              (`KismetSystemLibrary.PrintString` "Team1. Not enough minerals"))))))
    (:`NewEnumerator1`
      ;[1 1 1] Spawn Swordsman
      (bind _returnvalue_3 (`|GetDataTableRow` "/Game/Blueprints/Miscellaneous/CostsDataTable.CostsDataTable" "Swordsman")
        (:`then`
          (bind _bresult_2 (`/Game/Blueprints/KID_GameMode.RemoveEnergy` (`self.GameMode_Ref`) (`.Cost_5_B90C82224BB4A7B264F7EB84BBB7EBB3` (break `/Game/Blueprints/Miscellaneous/ESGameData` _returnvalue_3)) "Team1"))
          (if _bresult_2
            (bind _returnvalue_4 (`|SpawnActorFromClass` "/Game/Blueprints/Units/BP_Swordsman.BP_Swordsman_C" (`KismetMathLibrary.Conv_VectorToTransform` (`local.L_Position`)) "Undefined" "OverrideRootScale" null null))
            (`/Game/Blueprints/Units/BP_BaseCharacter.Initialize` _returnvalue_4 "Team1")
            (`KismetArrayLibrary.Array_Remove` (`self.SpawnEntitiesPool`))
            (else
              (`KismetSystemLibrary.PrintString` "Team1. Not enough minerals"))))))
    (:`NewEnumerator3`
      ;[1 1 1] Spawn Pikeman
      (bind _returnvalue_5 (`|GetDataTableRow` "/Game/Blueprints/Miscellaneous/CostsDataTable.CostsDataTable" "Swordsman")
        (:`then`
          (bind _bresult_3 (`/Game/Blueprints/KID_GameMode.RemoveEnergy` (`self.GameMode_Ref`) (`.Cost_5_B90C82224BB4A7B264F7EB84BBB7EBB3` (break `/Game/Blueprints/Miscellaneous/ESGameData` _returnvalue_5)) "Team1"))
          (if _bresult_3
            (bind _returnvalue_6 (`|SpawnActorFromClass` "/Game/Blueprints/Units/BP_Swordsman.BP_Swordsman_C" (`KismetMathLibrary.Conv_VectorToTransform` (`local.L_Position`)) "Undefined" "OverrideRootScale" null null))
            (`/Game/Blueprints/Units/BP_BaseCharacter.Initialize` _returnvalue_6 "Team1")
            (`KismetArrayLibrary.Array_Remove` (`self.SpawnEntitiesPool`))
            (else
              (`KismetSystemLibrary.PrintString` "Team1. Not enough minerals"))))))
    (:`NewEnumerator4`
      ;[1 1 1] Spawn Cavalry
      (bind _returnvalue_7 (`|GetDataTableRow` "/Game/Blueprints/Miscellaneous/CostsDataTable.CostsDataTable" "Archer")
        (:`then`
          (bind _bresult_4 (`/Game/Blueprints/KID_GameMode.RemoveEnergy` (`self.GameMode_Ref`) (`.Cost_5_B90C82224BB4A7B264F7EB84BBB7EBB3` (break `/Game/Blueprints/Miscellaneous/ESGameData` _returnvalue_7)) "Team1"))
          (if _bresult_4
            (bind _returnvalue_8 (`|SpawnActorFromClass` "/Game/Blueprints/Units/BP_Archer.BP_Archer_C" (`KismetMathLibrary.Conv_VectorToTransform` (`local.L_Position`)) "Undefined" "OverrideRootScale" null null))
            (`/Game/Blueprints/Units/BP_BaseCharacter.Initialize` _returnvalue_8 "Team1")
            (`KismetArrayLibrary.Array_Remove` (`self.SpawnEntitiesPool`))
            (else
              (`KismetSystemLibrary.PrintString` "Team1. Not enough minerals"))))))
    (:`NewEnumerator2`
      ;[1 1 1] Spawn Road
      (bind _returnvalue_9 (`|GetDataTableRow` "/Game/Blueprints/Miscellaneous/CostsDataTable.CostsDataTable" "Road")
        (:`then`
          (bind _bresult_5 (`/Game/Blueprints/KID_GameMode.RemoveEnergy` (`self.GameMode_Ref`) (`.Cost_5_B90C82224BB4A7B264F7EB84BBB7EBB3` (break `/Game/Blueprints/Miscellaneous/ESGameData` _returnvalue_9)) "Team1"))
          (if _bresult_5
            (set `/Game/Blueprints/Environment/BP_Tile.isConstructed` true _tiletospawn)
            (`/Game/Blueprints/Environment/BP_Tile.ShowTile` _tiletospawn)
            (`KismetArrayLibrary.Array_Remove` (`self.SpawnEntitiesPool`))
            (else
              (`KismetSystemLibrary.PrintString` "Team1. Not enough minerals"))))))
    (:`NewEnumerator5`
      ;[1 1 1] Spawn Tower
      (bind _returnvalue_10 (`|GetDataTableRow` "/Game/Blueprints/Miscellaneous/CostsDataTable.CostsDataTable" "Tower")
        (:`then`
          (bind _bresult_6 (`/Game/Blueprints/KID_GameMode.RemoveEnergy` (`self.GameMode_Ref`) (`.Cost_5_B90C82224BB4A7B264F7EB84BBB7EBB3` (break `/Game/Blueprints/Miscellaneous/ESGameData` _returnvalue_10)) "Team1"))
          (if _bresult_6
            (bind _returnvalue_11 (`|SpawnActorFromClass` "/Game/Blueprints/Buildings/BP_Tower.BP_Tower_C" (`KismetMathLibrary.MakeTransform` (`local.L_Position`)) "Undefined" "OverrideRootScale" null null))
            (`/Game/Blueprints/Buildings/BP_BaseBuilding.Initialize` _returnvalue_11 "Team1")
            (`KismetArrayLibrary.Array_Remove` (`self.SpawnEntitiesPool`))
            (else
              (`KismetSystemLibrary.PrintString` "Team1. Not enough minerals"))))))
    (:`NewEnumerator6`
      ;[1 1 1] Spawn Mine
      (bind _returnvalue_12 (`|GetDataTableRow` "/Game/Blueprints/Miscellaneous/CostsDataTable.CostsDataTable" "Mine")
        (:`then`
          (bind _bresult_7 (`/Game/Blueprints/KID_GameMode.RemoveEnergy` (`self.GameMode_Ref`) (`.Cost_5_B90C82224BB4A7B264F7EB84BBB7EBB3` (break `/Game/Blueprints/Miscellaneous/ESGameData` _returnvalue_12)) "Team1"))
          (if _bresult_7
            (bind _returnvalue_13 (`|SpawnActorFromClass` "/Game/Blueprints/Buildings/BP_Mine.BP_Mine_C" (`KismetMathLibrary.MakeTransform` (`local.L_Position`)) "Undefined" "OverrideRootScale" null null))
            (`/Game/Blueprints/Buildings/BP_BaseBuilding.Initialize` _returnvalue_13 "Team1")
            (`KismetArrayLibrary.Array_Remove` (`self.SpawnEntitiesPool`))
            (else
              (`KismetSystemLibrary.PrintString` "Team1. Not enough minerals"))))))))

(fn `GetMinePositionToSpawn`
  (returns (Position :type "Vector Structure"))
  (locals (L_Ties :type "Array of /Game/Blueprints/Environment/BP_Tile Object Reference") (L_TilesGood :type "Array of /Game/Blueprints/Environment/BP_Tile Object Reference"))
  (bind _l_tilesgood (`local.L_TilesGood`))
  (bind _output (`|GetArrayItem` _l_tilesgood (`KismetMathLibrary.RandomInteger` (`KismetArrayLibrary.Array_Length` _l_tilesgood))))
  (bind (_returnvalue_x _returnvalue_y _returnvalue_z) (`KismetMathLibrary.BreakVector` (`self.K2_GetActorLocation` _output)))
  (`KismetArrayLibrary.Array_Clear` (`local.L_Ties`))
  (`KismetArrayLibrary.Array_Clear` (`local.L_TilesGood`))
  (bind _outactors (`GameplayStatics.GetAllActorsOfClass` "/Game/Blueprints/Environment/BP_Tile.BP_Tile_C"))
  (bind _output_get (set `local.L_Ties` _outactors))
  (for _array_element _output_get
    (if (`/Game/Blueprints/Environment/BP_Tile.isConstructed` _array_element)
      (if (`/Game/Blueprints/Environment/BP_Tile.isMinerals` _array_element)
        (`KismetArrayLibrary.Array_Add` (`local.L_TilesGood`) _array_element))))
  (`/Engine/EditorBlueprintResources/StandardMacros.IsValid` _output
    (:`Is Valid`
      (return (`KismetMathLibrary.MakeVector` _returnvalue_x _returnvalue_y (+ _returnvalue_z 200.0))))))

(fn `GetTileToSpawn`
  (returns (Tile :type "/Game/Blueprints/Environment/BP_Tile Object Reference"))
  (locals (L_Tiles :type "Array of /Game/Blueprints/Environment/BP_Tile Object Reference"))
  (bind _l_tiles (`local.L_Tiles`))
  (bind _outactors (`GameplayStatics.GetAllActorsOfClass` "/Game/Blueprints/Environment/BP_Tile.BP_Tile_C"))
  (bind _output_get (set `local.L_Tiles` _outactors))
  (for (_array_element _array_index) _output_get
    (if (`/Game/Blueprints/Environment/BP_Tile.isConstructed` _array_element)
      (`KismetArrayLibrary.Array_Remove` (`local.L_Tiles`) _array_index)))
  (return (`|GetArrayItem` _l_tiles (`KismetMathLibrary.RandomInteger` (`KismetArrayLibrary.Array_Length` _l_tiles)))))

(fn `GetTowerPositionToSpawn`
  (returns (Position :type "Vector Structure"))
  (locals (L_Tiles :type "Array of /Game/Blueprints/Environment/BP_Tile Object Reference") (L_TilesGood :type "Array of /Game/Blueprints/Environment/BP_Tile Object Reference"))
  (bind _l_tilesgood (`local.L_TilesGood`))
  (bind _output (`|GetArrayItem` _l_tilesgood (`KismetMathLibrary.RandomInteger` (`KismetArrayLibrary.Array_Length` _l_tilesgood))))
  (bind (_returnvalue_x _returnvalue_y _returnvalue_z) (`KismetMathLibrary.BreakVector` (`self.K2_GetActorLocation` _output)))
  (`KismetArrayLibrary.Array_Clear` (`local.L_Tiles`))
  (`KismetArrayLibrary.Array_Clear` (`local.L_TilesGood`))
  (bind _outactors (`GameplayStatics.GetAllActorsOfClass` "/Game/Blueprints/Environment/BP_Tile.BP_Tile_C"))
  (bind _output_get (set `local.L_Tiles` _outactors))
  (for _array_element _output_get
    (if (`/Game/Blueprints/Environment/BP_Tile.isConstructed` _array_element)
      (if (`/Game/Blueprints/Environment/BP_Tile.bForTowerAI` _array_element)
        (`KismetArrayLibrary.Array_Add` (`local.L_TilesGood`) _array_element))))
  (`/Engine/EditorBlueprintResources/StandardMacros.IsValid` _output
    (:`Is Valid`
      (return (`KismetMathLibrary.MakeVector` _returnvalue_x _returnvalue_y (+ _returnvalue_z 200.0))))))

(fn `GetUnitPositionToSpawn`
  (returns (Position :type "Vector Structure"))
  (bind (_playerbs _team1bs) (`self.GetAllArrays`))
  (bind _output (`|GetArrayItem` _team1bs (`KismetMathLibrary.RandomInteger` (`KismetArrayLibrary.Array_Length` _team1bs))))
  (`/Engine/EditorBlueprintResources/StandardMacros.IsValid` _output
    (:`Is Valid`
      (bind (_returnvalue_x _returnvalue_y _returnvalue_z) (`KismetMathLibrary.BreakVector` (`self.K2_GetActorLocation` _output)))
      (return (`KismetMathLibrary.MakeVector` (- _returnvalue_x 400.0) _returnvalue_y (+ _returnvalue_z 100.0))))))

(fn `RollOrders`
  (returns (OrderNumber :type Integer))
  (locals (L_TotalWeights :type Integer) (L_WeightsArray :type "Array of Integer") (L_RandomValue :type Integer) (L_CurrentSum :type Integer) (L_OrderIndex :type Integer))
  (bind (_ordersweights_archer _ordersweights_swordsman _ordersweights_pikeman _ordersweights_cavalry _ordersweights_road _ordersweights_tower _ordersweights_mine) (break `/Game/Blueprints/Miscellaneous/ESOrderWeight` (`self.OrdersWeights`)))
  (bind _l_weightsarray (`local.L_WeightsArray`))
  (bind (_ordersweights_archer_2 _ordersweights_swordsman_2 _ordersweights_pikeman_2 _ordersweights_cavalry_2 _ordersweights_road_2 _ordersweights_tower_2 _ordersweights_mine_2) (break `/Game/Blueprints/Miscellaneous/ESOrderWeight` (`self.OrdersWeights`)))
  (bind _l_weightsarray_2 (`local.L_WeightsArray`))
  (bind _l_currentsum (`local.L_CurrentSum`))
  (`KismetArrayLibrary.Array_Clear` _l_weightsarray)
  (`|ExecutionSequence`
    (:`then_0`
      (`KismetArrayLibrary.Array_Add` _l_weightsarray _ordersweights_archer))
    (:`then_1`
      (`KismetArrayLibrary.Array_Add` _l_weightsarray _ordersweights_swordsman))
    (:`then_2`
      (`KismetArrayLibrary.Array_Add` _l_weightsarray _ordersweights_pikeman))
    (:`then_3`
      (`KismetArrayLibrary.Array_Add` _l_weightsarray _ordersweights_cavalry))
    (:`then_4`
      (`KismetArrayLibrary.Array_Add` _l_weightsarray _ordersweights_road))
    (:`then_5`
      (`KismetArrayLibrary.Array_Add` _l_weightsarray _ordersweights_tower))
    (:`then_6`
      (`KismetArrayLibrary.Array_Add` _l_weightsarray _ordersweights_mine)
      (bind _output_get (set `local.L_TotalWeights` (+ _ordersweights_archer_2 _ordersweights_swordsman_2 _ordersweights_pikeman_2 _ordersweights_cavalry_2 _ordersweights_road_2 _ordersweights_tower_2 _ordersweights_mine_2)))
      (set `local.L_RandomValue` (`KismetMathLibrary.RandomInteger` _output_get))
      (set `local.L_CurrentSum` (`|GetArrayItem` _l_weightsarray_2))
      (for (_array_element _array_index) _l_weightsarray_2
        (if (>= _l_currentsum (`local.L_RandomValue`))
          (set `local.L_OrderIndex` _array_index)
          (break)
          (else
            (set `local.L_CurrentSum` (+ _array_element _l_currentsum)))))
      (return (`local.L_OrderIndex`)))))

(fn `SpawnBuildings`)

(fn `UpdatePool`
  (locals (L_MaxThreatLvl :type "/Game/Blueprints/Miscellaneous/ESOrder Structure") (L_IndexOfMaxThreatLvlOrder :type Integer))
  (bind _spawnentitiespool (`self.SpawnEntitiesPool`))
  (bind _threatlevel (`self.ThreatLevel`))
  (bind _spawnentitiespool_2 (`self.SpawnEntitiesPool`))
  (if (not (== (`KismetArrayLibrary.Array_Length` (`self.SpawnEntitiesPool`)) 0))
    ;[1 1 1] remove order with threat lvl out of range
    (for _array_element (`self.SpawnEntitiesPool`)
      (bind (_spawntype _position _threatlvl _threatlvldelta) (break `/Game/Blueprints/Miscellaneous/ESOrder` _array_element))
      (if (not (`KismetMathLibrary.InRange_IntInt` _threatlvl (- _threatlevel _threatlvldelta) (+ _threatlevel _threatlvldelta)))
        (`KismetArrayLibrary.Array_RemoveItem` (`self.SpawnEntitiesPool`) _array_element)))
    ;[1 1 1] Get order with maximum threat level
    (set `local.L_IndexOfMaxThreatLvlOrder` 0)
    (set `local.L_MaxThreatLvl` (`|GetArrayItem` _spawnentitiespool))
    (for (_array_element_2 _array_index) _spawnentitiespool
      (if (>= (`.ThreatLvl_11_971100F74DC34FF632D69FADC8777604` (break `/Game/Blueprints/Miscellaneous/ESOrder` _array_element_2)) (`.ThreatLvl_11_971100F74DC34FF632D69FADC8777604` (break `/Game/Blueprints/Miscellaneous/ESOrder` (`local.L_MaxThreatLvl`))))
        (set `local.L_IndexOfMaxThreatLvlOrder` _array_index)
        (set `local.L_MaxThreatLvl` _array_element_2)))
    (`KismetArrayLibrary.Array_Remove` _spawnentitiespool_2 (`local.L_IndexOfMaxThreatLvlOrder`))
    (`KismetArrayLibrary.Array_Insert` _spawnentitiespool_2 (`local.L_MaxThreatLvl`))))

(fn `UserConstructionScript`)